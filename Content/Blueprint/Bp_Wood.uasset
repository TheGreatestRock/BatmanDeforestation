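; Bp_Wood is a wood item actor that the third-person character can pick up.
; It becomes carriable one second after BeginPlay, then passes itself to the character's Pickup function when an overlap begins.
; An unconnected graph fragment would set the cube's world scale from its relative scale while IsDropped is true, but it never runs.
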(event `self.ReceiveBeginPlay`
  (`KismetSystemLibrary.Delay` 1.0)
  (set `self.CanBeCarried` true))

(event `self.ReceiveActorBeginOverlap`
  (params (OtherActor :type "Actor Object Reference"))
  (if (`self.CanBeCarried`)
    (bind _asbp_third_person_character (cast `/Game/Blueprint/BP_ThirdPersonCharacter` OtherActor))
    (`/Game/Blueprint/BP_ThirdPersonCharacter.Pickup` _asbp_third_person_character self)))

(fn `UserConstructionScript`)