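; Spawner actor that periodically spawns SpawnClass at random points within its Box extent.
; StartSpawn starts a looping Cooldown timer that calls Spawn, which counts down from SpawnCount and clears the timer once below zero, yielding SpawnCount + 1 spawns.
; A negative SpawnCount spawns indefinitely.
; SnapToFloor uses a downward visibility trace and spawns at the hit location without checking for a hit.
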(event `StartSpawn`
  (set `self.ThingsToSpawn` (`self.SpawnCount`))
  (bind _returnvalue (`KismetSystemLibrary.K2_SetTimerDelegate` (delegate `Spawn`) (`self.Cooldown`) true true))
  (bind _output_get (set `self.Timer` _returnvalue)))

(event `Spawn`
  (bind _thingstospawn (`self.ThingsToSpawn`))
  (bind _spawnclass (`self.SpawnClass`))
  (bind _returnvalue (`KismetMathLibrary.RandomPointInBoundingBox` (`self.K2_GetActorLocation`) (`BoxComponent.BoxExtent` (`self.Box`))))
  (if (>= (`self.SpawnCount`) 0)
    (if (>= _thingstospawn 0)
      (`/Engine/EditorBlueprintResources/StandardMacros.DecrementInt` _thingstospawn
        (:`  `
          (if (`self.SnapToFloor`) :!label _label
            (bind _outhit (`KismetSystemLibrary.LineTraceSingle` (+ _returnvalue (`KismetMathLibrary.MakeVector` 0.0 0.0 (`self.SpawnHeightOffset`))) (- _returnvalue (0.0 0.0 10000.0)) "TraceTypeQuery1"))
            (`|SpawnActorFromClass` _spawnclass (`KismetMathLibrary.MakeTransform` (`.Location` (`GameplayStatics.BreakHitResult` _outhit))) "Undefined" "MultiplyWithRoot" null null)
            (else
              (`|SpawnActorFromClass` _spawnclass (`KismetMathLibrary.MakeTransform` _returnvalue) "Undefined" "MultiplyWithRoot" null null)))))
      (else
        (`KismetSystemLibrary.K2_InvalidateTimerHandle` (stale `StartSpawn` _output_get))))
    (else
      (goto _label))))

(fn `UserConstructionScript`)