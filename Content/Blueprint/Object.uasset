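; Toy actor that rides a spline, turns into a wrapped gift along the way and can then be picked up by the player.
; Once AddToSpline is called, Tick advances it along the spline, swapping mesh and scale at thresholds based on spline point 3.
; At the spline's end it stops moving and activates RotatingMovement.
; When carriable, overlapping BP_ThirdPersonCharacter increments its gift count and UI, then destroys the actor.
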(event `self.ReceiveActorBeginOverlap`
  (params (OtherActor :type "Actor Object Reference"))
  (if (`self.CanBeCarried`)
    (bind _asbp_third_person_character (cast `/Game/Blueprint/BP_ThirdPersonCharacter` OtherActor))
    (bind _result (`/Engine/EditorBlueprintResources/StandardMacros.IncrementInt` (`/Game/Blueprint/BP_ThirdPersonCharacter.GiftCarried` _asbp_third_person_character))
      (:`  `
        (set `/Game/Blueprint/WID_UI.NbToys` _result (`/Game/Blueprint/BP_ThirdPersonCharacter.UIWidget` _asbp_third_person_character))
        (`self.K2_DestroyActor`)))))

(event `self.ReceiveTick`
  (params (DeltaSeconds :type "Float (single-precision)"))
  (if (`self.IsOnSpline`)
    (`self.SplineMovement` DeltaSeconds)))

(fn `AddToSpline`
  (params (SplineActor :type "/Game/Blueprint/BP_Workshop Object Reference"))
  (set `self.SplineActor` SplineActor)
  (set `self.IsOnSpline` true))

(fn `OnFinishSpline`
  (set `self.IsOnSpline` false)
  (`ActorComponent.SetActive` (`self.RotatingMovement`) true true))

(fn `SplineMovement`
  (params (Tick :type "Float (double-precision)"))
  (bind _distance (`self.Distance`))
  (bind _mesh (`self.Mesh`))
  (bind _mesh_2 (`self.Mesh`))
  (bind _spline (`/Game/Blueprint/BP_Workshop.Spline` (`self.SplineActor`)))
  (bind _output_get (set `self.Distance` (+ _distance (* (`self.Speed`) Tick))))
  (if (< _distance (`SplineComponent.GetSplineLength` _spline))
    (bind _returnvalue (`SplineComponent.GetLocationAtDistanceAlongSpline` _spline _output_get "World"))
    (`self.K2_SetActorLocation` _returnvalue)
    (if (> (`SplineComponent.GetDistanceAlongSplineAtLocation` _spline _returnvalue "World") (/ (`SplineComponent.GetDistanceAlongSplineAtSplinePoint` _spline 3) 2.0))
      (bind _output_get_2 (set `self.CanBeCarried` (> (`SplineComponent.GetDistanceAlongSplineAtLocation` _spline _returnvalue "World") (* (`SplineComponent.GetDistanceAlongSplineAtSplinePoint` _spline 3) 1.1))))
      (if _output_get_2
        (`StaticMeshComponent.SetStaticMesh` _mesh "/Game/Assets/FBX/Cadeau_rouge2.Cadeau_rouge2")
        (`SceneComponent.SetRelativeScale3D` _mesh_2 (0.5 0.5 0.5))
        (else
          (`StaticMeshComponent.SetStaticMesh` _mesh "/Game/Assets/FBX/piti_cheval2.piti_cheval2")
          (`SceneComponent.SetRelativeScale3D` _mesh_2 (0.25 0.25 0.25)))))
    (else
      (`self.OnFinishSpline`))))

(fn `UserConstructionScript`)