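; Bp_Tree is a harvestable tree actor that loses health when damaged and drops wood when it is destroyed.
; TakeDamage plays a random-pitch hit sound, subtracts health and prints it, then at zero calls DropResource and destroys the tree.
; DropResource spawns one to three Bp_Wood actors with random offset and yaw, plus a break sound.
; After destruction, it calls StartSpawn on the Bp_Spawner child actor held by BP_ThirdPersonCharacter.
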(fn `Drop Resource`
  (bind _returnvalue (`self.GetTransform`))
  (for _ (range (+ (`KismetMathLibrary.RandomIntegerInRange` 1 3) 1))
    (`|SpawnActorFromClass` "/Game/Blueprint/Bp_Wood.Bp_Wood_C" (`KismetMathLibrary.MakeTransform` (+ (.location _returnvalue) (`KismetMathLibrary.MakeVector` (`KismetMathLibrary.Conv_IntToDouble` (`KismetMathLibrary.RandomIntegerInRange` -100 100)) (`KismetMathLibrary.Conv_IntToDouble` (`KismetMathLibrary.RandomIntegerInRange` -100 100)))) (`KismetMathLibrary.MakeRotator` (.roll (.rotation _returnvalue)) (.pitch (.rotation _returnvalue)) (`KismetMathLibrary.Conv_IntToDouble` (`KismetMathLibrary.RandomIntegerInRange` 0 360))) (.scale _returnvalue)) "Undefined" "MultiplyWithRoot" null null))
  (`GameplayStatics.PlaySoundAtLocation` "/Game/Assets/Wood_Explosion.Wood_Explosion" (`self.K2_GetActorLocation`) (struct) 2.5 (`KismetMathLibrary.RandomFloat`) 1.0 null null null null))

(fn `TakeDamage`
  (params (DamageAmount :type "Float (double-precision)"))
  (`GameplayStatics.PlaySoundAtLocation` "/Game/Assets/wood.wood" (`self.K2_GetActorLocation`) (struct) 5.0 (`KismetMathLibrary.RandomFloat`) 0.0 null null null null)
  (bind _output_get (set `self.Health` (- (`self.Health`) DamageAmount)))
  (`KismetSystemLibrary.PrintString` (`KismetStringLibrary.Conv_DoubleToString` _output_get))
  (if (<= _output_get 0.0)
    (`self.Drop Resource`)
    (`self.K2_DestroyActor`)
    (bind _returnvalue (`GameplayStatics.GetActorOfClass` "/Game/Blueprint/BP_ThirdPersonCharacter.BP_ThirdPersonCharacter_C"))
    (bind _asbp_spawner (cast `/Game/Blueprint/Bp_Spawner` (`ChildActorComponent.ChildActor` (`/Game/Blueprint/BP_ThirdPersonCharacter.Bp_Spawner` _returnvalue))))
    (`/Game/Blueprint/Bp_Spawner.StartSpawn` _asbp_spawner)))

(fn `UserConstructionScript`)